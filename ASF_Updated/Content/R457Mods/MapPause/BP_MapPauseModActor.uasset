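; Mod actor that pauses the game while the minimap is open and adds a manual pause toggle key.
; It binds to the player controller's minimap-open event and registers itself as a pauser through AskPauseStatic, checking PauseAsks for its own state.
; Closing the map restores the remembered manual pause unless MapOnly is set.
; MapOnly also limits the toggle to when the map is open or the mod already holds a pause.
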(event `self.ReceiveBeginPlay`
  (bind _asasfplayer_controller (cast `ASFPlayerController` (`GameplayStatics.GetPlayerController` 0)))
  (add `ASFPlayerController.OnMinimapOpenChanged` _asasfplayer_controller (delegate `ProcessOnMinimapOpenChanged`)))

(event `ProcessOnMinimapOpenChanged`
  (params (Controller :type "ASFPlayerController Object Reference") (Value :type Boolean))
  (if (`self.bMapOnly`)
    (`ASFPlayerController.AskPause_Static` self Value)
    (elif Value
      (`ASFPlayerController.AskPause_Static` self true)
      (else
        (`ASFPlayerController.AskPause_Static` self (`self.bWasManuallyPaused`))))))

(event `InputAction|ModPauseGame` :consume false
  (params (Key :type "Key Structure"))
  (:`Released`
    (bind _ballowed (`self.IsManualPauseAllowed`))
    (if _ballowed
      (bind _bispaused (`self.IsPausedByMod`))
      (bind _output_get (set `self.bWasManuallyPaused` (not _bispaused)))
      (`ASFPlayerController.AskPause_Static` self _output_get))))

(fn `IsManualPauseAllowed`
  (returns (bAllowed :type Boolean))
  (bind _asasfplayer_controller (cast `ASFPlayerController` (`GameplayStatics.GetPlayerController` 0))
    (:`then`
      (bind _returnvalue (`ASFPlayerController.IsInMinimap` _asasfplayer_controller))
      (return (or (not (`self.bMapOnly`)) _returnvalue (and (not _returnvalue) (`KismetArrayLibrary.Array_Contains` (`ASFPlayerController.Pause_Asks` _asasfplayer_controller) self)))))
    (:`CastFailed`
      (return false))))

(fn `IsPausedByMod`
  (returns (bIsPaused :type Boolean))
  (bind _asasfplayer_controller (cast `ASFPlayerController` (`GameplayStatics.GetPlayerController` 0))
    (:`then`
      (return (`KismetArrayLibrary.Array_Contains` (`ASFPlayerController.Pause_Asks` _asasfplayer_controller) self)))
    (:`CastFailed`
      (return false))))

(fn `UserConstructionScript`)