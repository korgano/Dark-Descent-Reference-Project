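; BP_NoDeathClockModActor is a mod actor that neutralizes the base-management death clock by holding its time allotment at 999.
; Tick feeds a 10-second Delay, so ModNoDeathClockSetTurns runs periodically rather than every frame.
; That function reads the current allotment from the base-management game state and passes any difference from 999 to the game mode's update function.
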(event `self.ReceiveTick`
  (params (DeltaSeconds :type "Float (single-precision)"))
  (`KismetSystemLibrary.Delay` 10.0)
  (`self.ModNoDeathClockSetTurns`))

(fn `ModNoDeathClockSetTurns`
  (bind _asasfgame_mode_base_base_management (cast `ASFGameModeBase_BaseManagement` (`GameplayStatics.GetGameMode`)))
  (bind _asasfgame_state_base_management (cast `ASFGameState_BaseManagement` (`GameplayStatics.GetGameState`)))
  (bind _returnvalue (- 999 (`ASFGameState_BaseManagement.CurrentDeathClockTimeAllotment` _asasfgame_state_base_management)))
  (if (!= _returnvalue 0)
    (`ASFGameModeBase_BaseManagement.UpdateCurrentDeathClockTimeAllotment` _asasfgame_mode_base_base_management _returnvalue)))

(fn `UserConstructionScript`)