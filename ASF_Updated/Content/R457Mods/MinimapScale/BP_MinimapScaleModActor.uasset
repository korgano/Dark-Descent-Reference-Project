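; Mod actor that rescales, repositions and sets the opacity of the tactical-mode motion tracker minimap widget.
; Each tick, Init finds the last WBP_TM_MotionTracker and climbs through its VerticalBox to the parent canvas slot, caching both.
; Once both are valid, ScaleMinimap applies the configured values a single time.
; The mission-loaded event on the tactical game mode clears the cached references so the tweak reapplies.
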(event `self.ReceiveTick`
  (params (DeltaSeconds :type "Float (single-precision)"))
  (`self.Init`)
  (if (`self.bWasInitialized`)
    (if (not (`self.bWasRescaled`))
      (`self.ScaleMinimap`)
      (set `self.bWasRescaled` true))
    (else
      (set `self.bWasRescaled` false))))

(event `self.ReceiveBeginPlay`
  (bind _asasfgame_mode_base_tactical_mode (cast `ASFGameModeBase_TacticalMode` (`GameplayStatics.GetGameMode`)))
  (add `ASFGameModeBase_TacticalMode.OnMissionLoaded` _asasfgame_mode_base_tactical_mode (delegate `InvalidateAllVars`)))

(event `InvalidateAllVars`
  (params (GameMode :type "ASFGameModeBase_TacticalMode Object Reference"))
  (set `self.MinimapWidget` null)
  (set `self.MinimapParentCanvas` null)
  (set `self.bWasInitialized` false)
  (set `self.bWasRescaled` false))

(fn `GetMinimapParentCanvas`
  (params (MinimapWidget :type "/Game/Blueprint/GUI/TacticalMission/MotionTracker/WBP_TM_MotionTracker Object Reference"))
  (returns (ParentCanvas :type "CanvasPanelSlot Object Reference"))
  (bind _asvertical_box_slot (cast `VerticalBoxSlot` (`Widget.Slot` MinimapWidget))
    (:`then`
      (bind _asvertical_box (cast `VerticalBox` (`KismetSystemLibrary.GetOuterObject` _asvertical_box_slot))
        (:`then`
          (bind _ascanvas_panel_slot (cast `CanvasPanelSlot` (`Widget.Slot` _asvertical_box))
            (:`then`
              (return _ascanvas_panel_slot))
            (:`CastFailed`
              _)))
        (:`CastFailed`
          _)))
    (:`CastFailed`
      _))
  (return null))

(fn `Init`
  (`/Engine/EditorBlueprintResources/StandardMacros.IsValid` (`self.MinimapWidget`)
    (:`Is Valid`
      (`/Engine/EditorBlueprintResources/StandardMacros.IsValid` (`self.MinimapParentCanvas`) :!label _label
        (:`Is Valid`
          (set `self.bWasInitialized` true :!label _label_2))
        (:`Is Not Valid`
          (bind _parentcanvas (`self.GetMinimapParentCanvas` (`self.MinimapWidget`)))
          (bind _output_get (set `self.MinimapParentCanvas` _parentcanvas))
          (`/Engine/EditorBlueprintResources/StandardMacros.IsValid` _output_get
            (:`Is Valid`
              (goto _label_2))
            (:`Is Not Valid`
              (set `self.bWasInitialized` false))))))
    (:`Is Not Valid`
      (bind _foundwidgets (`WidgetBlueprintLibrary.GetAllWidgetsOfClass` "/Game/Blueprint/GUI/TacticalMission/MotionTracker/WBP_TM_MotionTracker.WBP_TM_MotionTracker_C" false))
      (bind _output_get_2 (set `self.MinimapWidget` (`|GetArrayItem` _foundwidgets (`KismetArrayLibrary.Array_LastIndex` _foundwidgets))))
      (`/Engine/EditorBlueprintResources/StandardMacros.IsValid` _output_get_2
        (:`Is Valid`
          (goto _label))
        (:`Is Not Valid`
          (set `self.bWasInitialized` false))))))

(fn `ScaleMinimap`
  (bind _minimapscale (`self.MinimapScale`))
  (`Widget.SetRenderScale` (`self.MinimapWidget`) (`KismetMathLibrary.MakeVector2D` _minimapscale _minimapscale))
  (`CanvasPanelSlot.SetPosition` (`self.MinimapParentCanvas`) (`self.MinimapPosOffset`))
  (`Widget.SetRenderOpacity` (`self.MinimapWidget`) (`self.MinimapOpacity`)))

(fn `UserConstructionScript`)