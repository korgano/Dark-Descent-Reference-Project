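; Mod actor that shows marine name widgets for the player's squad while slow motion is active.
; A looping timer searches for the player Squad until found, then stops.
; Tick polls the player controller's SlowMoAsks, creating a UMG_MarineName per squad member on entry and removing them on exit.
; A skill-menu binding and a pause check are present but unused.
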(event `self.ReceiveBeginPlay`
  (bind _returnvalue (`KismetSystemLibrary.K2_SetTimerDelegate` (delegate `Init`) 1.0 true)))

(event `Init`
  (bind _bfound (`self.FindPlayerSquad`))
  (if _bfound
    (`KismetSystemLibrary.K2_ClearAndInvalidateTimerHandle` (stale `self.ReceiveBeginPlay` _returnvalue))))

(event `ShowHideNames`
  (params (Controller :type "ASFPlayerController Object Reference") (Value :type Boolean))
  (if Value
    (`self.InitWidgets`)
    (else
      (`self.CleanupWidgets`))))

(event `self.ReceiveTick`
  (params (DeltaSeconds :type "Float (single-precision)"))
  (bind _bresult (`self.IsInSlowMoOrPause`))
  (if _bresult
    (if (not (`self.bShowingNames`))
      (`self.InitWidgets`)
      (set `self.bShowingNames` true))
    (elif (`self.bShowingNames`)
      (`self.CleanupWidgets`)
      (set `self.bShowingNames` false))))

(fn `CleanupWidgets`
  (bind _namewidgets (`self.NameWidgets`))
  (for _array_element _namewidgets
    (`Widget.RemoveFromParent` _array_element))
  (`KismetArrayLibrary.Array_Clear` _namewidgets))

(fn `FindPlayerSquad`
  (returns (bFound :type Boolean))
  (bind _outactors (`GameplayStatics.GetAllActorsOfClass` "/Script/ASF.Squad"))
  (for _array_element _outactors
    (if (`Squad.IsPlayerSquad` _array_element)
      (set `self.PlayerSquad` _array_element)
      (return true)))
  (return false))

(fn `InitWidgets`
  (for _array_element (`Squad.GetSquadMembers` (`self.PlayerSquad`))
    (bind _returnvalue (`|CreateWidget` "/Game/R457Mods/MarineNames/UMG_MarineName.UMG_MarineName_C"))
    (`/Game/R457Mods/MarineNames/UMG_MarineName.Init` _returnvalue _array_element)
    (`UserWidget.AddToViewport` _returnvalue 0)
    (`KismetArrayLibrary.Array_Add` (`self.NameWidgets`) _returnvalue)))

(fn `IsInSlowMoOrPause`
  (returns (bResult :type Boolean))
  (bind _asasfplayer_controller (cast `ASFPlayerController` (`ASFGameplayStaticsLibrary.GetASFPlayerController`))
    (:`then`
      (return (> (`KismetArrayLibrary.Array_Length` (`ASFPlayerController.SlowMo_Asks` _asasfplayer_controller)) 0)))
    (:`CastFailed`
      (return false))))

(fn `UserConstructionScript`)