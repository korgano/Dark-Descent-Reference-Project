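; Mod loader actor that discovers R457 mods and spawns their mod actors for the current game layer.
; On BeginPlay it builds conventional /Game/R457Mods paths from ModsToLoad and blocking-loads each R457ModInfo asset.
; On the welcome screen it lists mod names in a UMG widget; otherwise it spawns actors for mods flagged for the active tactical or strategic layer.
; Spawned actors are tracked and destroyed on EndPlay.
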(event `self.ReceiveBeginPlay`
  (`self.Cleanup`)
  (`self.ScanForMods`)
  (bind _asbp_r457game_instance (cast `/Game/R457ModLoader/BP_R457GameInstance` (`GameplayStatics.GetGameInstance`)))
  (bind _bresult (`/Game/R457ModLoader/BP_R457GameInstance.IsInWelcomeScreen` _asbp_r457game_instance))
  (if _bresult
    (bind _returnvalue (`|CreateWidget` "/Game/R457ModLoader/UMG_LoaderModList.UMG_LoaderModList_C"))
    (`UserWidget.AddToViewport` _returnvalue 0)
    (for _array_element (`self.ModInfos`)
      (`/Game/R457ModLoader/UMG_LoaderModList.AddItem` _returnvalue (`/Game/R457ModLoader/R457ModInfo.ModFriendlyName` _array_element)))
    (else
      (for _array_element_2 (`self.ModInfos`)
        (bind _bshouldspawn (`self.ShouldSpawnThisMod` _array_element_2))
        (if _bshouldspawn
          (`self.SpawnNewModActor` (`/Game/R457ModLoader/R457ModInfo.ModActorToSpawn` _array_element_2)))))))

(event `self.ReceiveEndPlay`
  (params (EndPlayReason :type "EEndPlayReason Enum" :default "Destroyed"))
  (`self.Cleanup`))

(fn `BuildSoftPath`
  (params (ModName :type String))
  (returns (SoftObjPath :type "SoftObjectPath Structure"))
  (return (`KismetSystemLibrary.MakeSoftObjectPath` (`KismetStringLibrary.Concat_StrStr` "/Game/R457Mods/" ModName "/" ModName "ModInfo." ModName "ModInfo"))))

(fn `Cleanup`
  (for _array_element (`self.SpawnedModActors`)
    (`self.K2_DestroyActor` _array_element))
  (`KismetArrayLibrary.Array_Clear` (`self.SpawnedModActors`)))

(fn `ScanForMods`
  (for _array_element (`self.ModsToLoad`)
    (bind _softobjpath (`self.BuildSoftPath` _array_element))
    (`KismetArrayLibrary.Array_AddUnique` (`self.SoftPaths`) _softobjpath))
  (for _array_element_2 (`self.SoftPaths`)
    (bind _returnvalue (`KismetSystemLibrary.LoadAsset_Blocking` (`KismetSystemLibrary.Conv_SoftObjPathToSoftObjRef` _array_element_2)))
    (bind _asr457mod_info (cast `/Game/R457ModLoader/R457ModInfo` _returnvalue))
    (`KismetArrayLibrary.Array_AddUnique` (`self.ModInfos`) _asr457mod_info)))

(fn `ShouldSpawnThisMod`
  (params (ThisModInfo :type "/Game/R457ModLoader/R457ModInfo Object Reference"))
  (returns (bShouldSpawn :type Boolean))
  (bind _asbp_r457game_instance (cast `/Game/R457ModLoader/BP_R457GameInstance` (`GameplayStatics.GetGameInstance`))
    (:`then`
      (bind _bresult (`/Game/R457ModLoader/BP_R457GameInstance.IsInStrategicLayer` _asbp_r457game_instance))
      (bind _bresult_2 (`/Game/R457ModLoader/BP_R457GameInstance.IsInTacticalLayer` _asbp_r457game_instance))
      (return (and (or (and _bresult_2 (`/Game/R457ModLoader/R457ModInfo.bIsTacticalLayerMod` ThisModInfo)) (and _bresult (`/Game/R457ModLoader/R457ModInfo.bIsStrategicLayerMod` ThisModInfo))) (`KismetSystemLibrary.IsValidClass` (`/Game/R457ModLoader/R457ModInfo.ModActorToSpawn` ThisModInfo)))))
    (:`CastFailed`
      (return false))))

(fn `SpawnNewModActor`
  (params (ActorClass :type "Actor Class Reference"))
  (returns (SpawnedActor :type "Actor Object Reference"))
  (bind _returnvalue (`|SpawnActorFromClass` ActorClass (`KismetMathLibrary.MakeTransform` (0.0 0.0 0.0)) "AlwaysSpawn" "OverrideRootScale" null null))
  (`KismetArrayLibrary.Array_Add` (`self.SpawnedModActors`) _returnvalue)
  (return _returnvalue))

(fn `UserConstructionScript`)