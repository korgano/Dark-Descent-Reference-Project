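; Game instance for the R457 mod loader that keeps a mod actor spawner alive and announces game layer changes.
; A looping one-second timer detects game mode changes, fires welcome screen, base management or tactical notifications, and respawns BP_R457ModActorSpawner.
; The welcome screen also shows a loader message widget, and pawn controller changes are relayed through their own call.
; Helper functions report whether the current layer is welcome screen, strategic or tactical.
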(event `self.ReceiveInit`
  (`parent.ReceiveInit`)
  (add `GameInstance.OnPawnControllerChangedDelegates` (delegate `R457OnPawnControllerChanged`))
  (`KismetSystemLibrary.K2_SetTimerDelegate` (delegate `R457LoaderTimer`) 1.0 true))

(event `R457OnPawnControllerChanged`
  (params (Pawn :type "Pawn Object Reference") (Controller :type "Controller Object Reference"))
  (`self.R457PawnControllerChanged`))

(event `R457LoaderTimer`
  (bind _returnvalue (`GameplayStatics.GetGameMode`))
  (if (`self.bGameModeChangeHandled`)
    (`/Engine/EditorBlueprintResources/StandardMacros.IsValid` (`self.ModSpawner`)
      (:`Is Valid`
        _)
      (:`Is Not Valid`
        (`self.InitModSpawner`))))
  (`self.CheckGameModeChanged`)
  (if (not (`self.bGameModeChangeHandled`))
    (cast `/Game/Blueprint/GameData/GameMode/BP_ASFGameModeWelcomeScreen` _returnvalue
      (:`then`
        (`self.R457ChangedToWelcomeScreen`)
        (bind _returnvalue_2 (`|CreateWidget` "/Game/R457ModLoader/UMG_LoaderMessage.UMG_LoaderMessage_C"))
        (`UserWidget.AddToViewport` _returnvalue_2 0))
      (:`CastFailed`
        (cast `ASFGameModeBase_BaseManagement` _returnvalue
          (:`then`
            (`self.R457ChangedToBaseManagement`))
          (:`CastFailed`
            (cast `/Game/Blueprint/GameData/GameMode/BP_ASFGameModeBase_TacticalMode` _returnvalue)
            (`self.R457ChangedToTacticalMode`)))))
    (`self.InitModSpawner`)
    (set `self.bGameModeChangeHandled` true)))

(fn `CheckGameModeChanged`
  (if (!= (`GameplayStatics.GetGameMode`) (`self.SavedGameMode`))
    (set `self.SavedGameMode` (`GameplayStatics.GetGameMode`))
    (set `self.bGameModeChangeHandled` false)))

(fn `InitModSpawner`
  (bind _outactors (`GameplayStatics.GetAllActorsOfClass` "/Game/R457ModLoader/BP_R457ModActorSpawner.BP_R457ModActorSpawner_C"))
  (for _array_element _outactors
    (`Actor.K2_DestroyActor` _array_element))
  (bind _returnvalue (`|SpawnActorFromClass` "/Game/R457ModLoader/BP_R457ModActorSpawner.BP_R457ModActorSpawner_C" (`KismetMathLibrary.MakeTransform` (0.0 0.0 0.0)) "AlwaysSpawn" "OverrideRootScale" null null))
  (set `self.ModSpawner` _returnvalue))

(fn `IsInStrategicLayer`
  (returns (bResult :type Boolean))
  (cast `ASFGameModeBase_BaseManagement` (`GameplayStatics.GetGameMode`)
    (:`then`
      (return true))
    (:`CastFailed`
      (return false))))

(fn `IsInTacticalLayer`
  (returns (bResult :type Boolean))
  (cast `/Game/Blueprint/GameData/GameMode/BP_ASFGameModeBase_TacticalMode` (`GameplayStatics.GetGameMode`)
    (:`then`
      (return true))
    (:`CastFailed`
      (return false))))

(fn `IsInWelcomeScreen`
  (returns (bResult :type Boolean))
  (cast `/Game/Blueprint/GameData/GameMode/BP_ASFGameModeWelcomeScreen` (`GameplayStatics.GetGameMode`)
    (:`then`
      (return true))
    (:`CastFailed`
      (return false))))